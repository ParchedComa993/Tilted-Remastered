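; BP_FragmentPiece is a rune fragment sprite that plays a timed vanishing effect when its Box is overlapped, then destroys itself.
; A chain of Delays steps the RuneSpin rotation rate ever faster while the FBRuneFragment sprite brightens, turns more transparent and scales down from a slight swell.
; The overlap does not filter the other actor, and no collection or reward logic runs here.
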(event `self.Box.OnComponentBeginOverlap`
  (params (OverlappedComponent :type "PrimitiveComponent Object Reference") (OtherActor :type "Actor Object Reference") (OtherComp :type "PrimitiveComponent Object Reference") (OtherBodyIndex :type Integer) (bFromSweep :type Boolean) (SweepResult :type "HitResult Structure (by ref)"))
  (bind _fb_runefragment (`self.FB_RuneFragment`))
  (bind _fb_runefragment_2 (`self.FB_RuneFragment`))
  (bind _fb_runefragment_3 (`self.FB_RuneFragment`))
  (bind _fb_runefragment_4 (`self.FB_RuneFragment`))
  (`KismetSystemLibrary.Delay` 0.2)
  (set `RotatingMovementComponent.RotationRate` (struct :`Pitch` 45.0) (`self.RuneSpin`))
  (`PaperFlipbookComponent.SetSpriteColor` _fb_runefragment_2 (struct :`R` 0.541667 :`G` 0.541667 :`B` 0.541667 :`A` 0.8))
  (`SceneComponent.SetWorldScale3D` _fb_runefragment_2 (1.1 1.0 1.1))
  (`KismetSystemLibrary.Delay` 0.5)
  (set `RotatingMovementComponent.RotationRate` (struct :`Pitch` 90.0) (`self.RuneSpin`))
  (`PaperFlipbookComponent.SetSpriteColor` _fb_runefragment_3 (struct :`R` 0.727431 :`G` 0.727431 :`B` 0.727431 :`A` 0.7))
  (`SceneComponent.SetWorldScale3D` _fb_runefragment_3 (0.9 1.0 0.9))
  (`KismetSystemLibrary.Delay` 1.0)
  (set `RotatingMovementComponent.RotationRate` (struct :`Pitch` 180.0) (`self.RuneSpin`))
  (`PaperFlipbookComponent.SetSpriteColor` _fb_runefragment_4 (struct :`R` 0.838542 :`G` 0.838542 :`B` 0.838542 :`A` 0.6))
  (`SceneComponent.SetWorldScale3D` _fb_runefragment_4 (0.7 1.0 0.7))
  (`KismetSystemLibrary.Delay` 1.5)
  (set `RotatingMovementComponent.RotationRate` (struct :`Pitch` 360.0) (`self.RuneSpin`))
  (`PaperFlipbookComponent.SetSpriteColor` _fb_runefragment (struct :`R` 0.869792 :`G` 0.869792 :`B` 0.869792 :`A` 0.5))
  (`SceneComponent.SetWorldScale3D` _fb_runefragment (0.3 1.0 0.3))
  (`KismetSystemLibrary.Delay` 2.0)
  (set `RotatingMovementComponent.RotationRate` (struct :`Pitch` 720.0) (`self.RuneSpin`))
  (`PaperFlipbookComponent.SetSpriteColor` (`self.FB_RuneFragment`) (struct :`R` 1.0 :`G` 1.0 :`B` 1.0 :`A` 0.4))
  (`KismetSystemLibrary.Delay` 3.0)
  (`self.K2_DestroyActor`))

(fn `UserConstructionScript`)